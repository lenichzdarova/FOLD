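; BP_GroupTest is a test Blueprint that assigns placeholder party membership to connected players.
; Shortly after BeginPlay, the server loops over the GameState's PlayerArray and casts each entry to FOLDPlayerStateBase.
; It sets each player's PlayerParty member IDs to that player's array index as a string plus a hardcoded second ID.
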(event `self.ReceiveBeginPlay`
  (`KismetSystemLibrary.Delay` 2.0)
  (if (`KismetSystemLibrary.IsServer`)
    (for (_array_element _array_index) (`GameStateBase.PlayerArray` (`GameplayStatics.GetGameState`))
      (bind _asfoldplayer_state_base (cast `FOLDPlayerStateBase` _array_element))
      (`PlayerParty.SetPartyMembersID` (`FOLDPlayerStateBase.PlayerParty` _asfoldplayer_state_base) (`|MakeArray` (`KismetStringLibrary.Conv_IntToString` _array_index) "2")))))

(fn `UserConstructionScript`)