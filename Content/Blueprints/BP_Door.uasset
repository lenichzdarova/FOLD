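; BP_Door is an interactable door that toggles between open and closed on each Interact event.
; Open and Close instantly set the Scene component's relative rotation, swinging it to a 90-degree yaw or back to zero, with no animation.
; The door stores no state variable, as IsOpened treats any non-zero yaw on that component as open.
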(event `self.Interact`
  (params (interactor :type "CharacterBase Object Reference"))
  (if (`self.IsOpened`)
    (`self.Close`)
    (else
      (`self.Open`))))

(fn `Close`
  (`SceneComponent.K2_SetRelativeRotation` (`self.Scene`) (struct) false false))

(fn `IsOpened`
  (returns (bIsOpen :type Boolean))
  (bind (_relativerotation_roll _relativerotation_pitch _relativerotation_yaw) (`KismetMathLibrary.BreakRotator` (`SceneComponent.RelativeRotation` (`self.Scene`))))
  (return (!= _relativerotation_yaw 0.0)))

(fn `Open`
  (`SceneComponent.K2_SetRelativeRotation` (`self.Scene`) (struct :`Yaw` 90.0) false false))

(fn `UserConstructionScript`)