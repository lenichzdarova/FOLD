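; BP_TestGrid is a debug Blueprint for previewing the grid built by the navigation subsystem.
; On BeginPlay it sets the subsystem's cell size, passes itself to SetupGrid and shows the test grid.
; The TestGrid event repeats the setup and display without resetting the cell size, while Flush clears persistent debug lines.
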(event `self.ReceiveBeginPlay`
  (bind _returnvalue (subsystem `NavigationSubsystem`))
  (set `NavigationSubsystem.CellSize` 100.0 (subsystem `NavigationSubsystem`))
  (`NavigationSubsystem.SetupGrid` _returnvalue self)
  (`NavigationSubsystem.ShowTestGrid` _returnvalue))

(event `Flush`
  (`KismetSystemLibrary.FlushPersistentDebugLines`))

(event `TestGrid`
  (bind _returnvalue (subsystem `NavigationSubsystem`))
  (`NavigationSubsystem.SetupGrid` _returnvalue self)
  (`NavigationSubsystem.ShowTestGrid` _returnvalue))

(fn `UserConstructionScript`)