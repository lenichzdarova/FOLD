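; Player controller Blueprint that sets up the player's view, character entity, input and UI when play begins.
; BeginPlay spawns PlayerView and CharacterEntity at the world origin, makes PlayerView the view target and adds the IMC_InputMapping Enhanced Input context.
; It then calls SetupWidgets, which creates and stores the down panel widget without adding it to the viewport, and SetupStates.
; The IA_Action input event is an empty stub.
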(event `self.ReceiveBeginPlay`
  (bind _returnvalue (`KismetMathLibrary.Conv_VectorToTransform` (`KismetMathLibrary.Vector_Zero`)))
  (bind _returnvalue_2 (`|SpawnActorFromClass` "/Script/FalloutOld.PlayerView" _returnvalue "Undefined" "MultiplyWithRoot" null null))
  (set `self.PlayerView` _returnvalue_2)
  (bind _returnvalue_3 (`|SpawnActorFromClass` "/Script/FalloutOld.CharacterEntity" _returnvalue "Undefined" "MultiplyWithRoot" null null))
  (set `self.PlayerCharacter` _returnvalue_3)
  (`self.SetViewTargetWithBlend` (`self.PlayerView`))
  (`EnhancedInputSubsystemInterface.AddMappingContext` (pcsubsystem `EnhancedInputLocalPlayerSubsystem` self) "/Game/Blueprints/Input/IMC_InputMapping.IMC_InputMapping" 0 (struct))
  (`self.SetupWidgets`)
  (`self.SetupStates`))

(event `EnhancedInput|/Game/Blueprints/Input/IA_Action`
  (params (ActionValue :type Boolean) (ElapsedSeconds :type "Float (double-precision)") (TriggeredSeconds :type "Float (double-precision)") (InputAction :type "InputAction Object Reference" :default "/Game/Blueprints/Input/IA_Action.IA_Action")))

(fn `SetupWidgets`
  (bind _returnvalue (`|CreateWidget` "/Game/Blueprints/UI/WBP_DownPanel.WBP_DownPanel_C"))
  (set `self.UWidgetDownPanel` _returnvalue))

(fn `UserConstructionScript`)